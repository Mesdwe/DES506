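; PurifyWaterTrigger is a one-shot location trigger that unlocks an invocation entry in the player's Grimoire.
; A BeginOverlap flag selects whether it fires when the FirstPersonCharacter enters or leaves its Box volume.
; It passes the InvocationInfo title to the character's GrimoireComponent, marked as a trigger unlock, then destroys itself.
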(event OnComponentBeginOverlap(Box)
  (params (OverlappedComponent :type Primitive%20Component%20Object%20Reference) (OtherActor :type Actor%20Object%20Reference) (OtherComp :type Primitive%20Component%20Object%20Reference) (OtherBodyIndex :type Integer) (bFromSweep :type Boolean) (SweepResult :type Hit%20Result%20Structure%20%28by%20ref%29))
  (if (Variables|Default|GetBeginOverlap)
    (bind _asfirst_person_character (Utilities|Casting|CastToFirstPersonCharacter OtherActor))
    (Default|UnlockInvocationEntry (Variables|/Game/Blueprints/FirstPersonCharacter.FirstPersonCharacter_C|GetGrimoireComponent _asfirst_person_character) (.Title (Utilities|Struct|BreakInvocation (Variables|Default|GetInvocationInfo))) true)
    (Actor|DestroyActor)))

(event OnComponentEndOverlap(Box)
  (params (OverlappedComponent :type Primitive%20Component%20Object%20Reference) (OtherActor :type Actor%20Object%20Reference) (OtherComp :type Primitive%20Component%20Object%20Reference) (OtherBodyIndex :type Integer))
  (if (not (Variables|Default|GetBeginOverlap))
    (bind _asfirst_person_character (Utilities|Casting|CastToFirstPersonCharacter OtherActor))
    (Default|UnlockInvocationEntry (Variables|/Game/Blueprints/FirstPersonCharacter.FirstPersonCharacter_C|GetGrimoireComponent _asfirst_person_character) (.Title (Utilities|Struct|BreakInvocation (Variables|Default|GetInvocationInfo))) true)
    (Actor|DestroyActor)))

(fn ConstructionScript)