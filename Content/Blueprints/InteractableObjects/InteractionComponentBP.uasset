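; Interaction component that detects objects the player looks at and shows an interaction icon for interactable ones.
; Each tick it line-traces from the first-person camera on the Visibility channel and checks the hit actor for the PlayerInteract interface.
; A DoOnce gates the focus message and widget creation.
; Looking away removes the widget and clears the stored actor before sending it the look-away message, so that call targets None.
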(event Custom|ChangeCursor
  (params (Hovered :type Boolean) (Interactable :type Boolean))
  ;[1 1 1] Display UI
  (if (and Hovered Interactable)
    (bind _returnvalue (UserInterface|CreateWidget "/Game/Blueprints/UI/ObjectInteraction_WID.ObjectInteraction_WID_C"))
    (UserInterface|Viewport|AddtoViewport _returnvalue 0)
    (Variables|Default|SetIconRef _returnvalue)
    (else
      (bind _iconref (Variables|Default|GetIconRef)
        (:then
          (Widget|RemovefromParent _iconref)
          (Variables|Default|SetIconRef 0)
          (Variables|Default|SetBeforeActor 0))
        (:else)))))

(event EventBeginPlay
  (bind _asfirst_person_character (Utilities|Casting|CastToFirstPersonCharacter (Game|GetPlayerCharacter 0)))
  (Variables|Default|SetFirst%20Person%20Camera%20Component (Variables|/Script/Sludge.SludgeCharacter|GetFirstPersonCameraComponent _asfirst_person_character)))

(event EventTick
  (params (DeltaSeconds :type Float%20%28single-precision%29))
  (bind _first_person_camera_component (Variables|Default|GetFirst%20Person%20Camera%20Component))
  (bind _returnvalue (Transformation|GetWorldLocation _first_person_camera_component))
  (bind _outhit (Collision|LineTraceByChannel _returnvalue (+ _returnvalue (* (Math|Vector|GetForwardVector _first_person_camera_component) 1e+03)) "TraceTypeQuery1" false 0 "None"))
  (if (Utilities|DoesObjectImplementInterface (.HitActor (Collision|BreakHitResult _outhit)) "/Script/Sludge.PlayerInteract")
    (if (== (Variables|Default|GetBeforeActor) 0)
      (bind _returnvalue_2 (Class|PlayerInteract|GetInteractable(Message) (.HitActor (Collision|BreakHitResult _outhit))))
      (if _returnvalue_2
        (Utilities|FlowControl|DoOnce false :!label _label
          (:Completed
            (Class|PlayerInteract|OnFocus(Message) (.HitActor (Collision|BreakHitResult _outhit)))
            (bind _output_get (Variables|Default|SetBeforeActor (.HitActor (Collision|BreakHitResult _outhit))))
            (bind _returnvalue_3 (Class|PlayerInteract|GetInteractable(Message) _output_get))
            (CallFunction|ChangeCursor true _returnvalue_3)))
        (else
          (goto _label Reset)))
      (else
        (goto _label Reset)))
    (elif (!= (.HitActor (Collision|BreakHitResult _outhit)) (Variables|Default|GetBeforeActor))
      (CallFunction|ChangeCursor false false)
      (Variables|Default|SetBeforeActor 0)
      (Class|PlayerInteract|LookAway(Message) (Variables|Default|GetBeforeActor))
      (goto _label Reset))))