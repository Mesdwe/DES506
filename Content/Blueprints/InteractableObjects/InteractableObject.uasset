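; Base interactable world object that unlocks its journal entry in the player's Grimoire component when first interacted with, then becomes non-interactable.
; BeginPlay feeds the static mesh and exposed particle settings into a Niagara glow effect.
; Interaction VFX either stops spawning and boosts brightness, or shifts glow color through a timeline, depending on KillOnGet.
; A separate DisplayUI event creates a new-entry widget or resets its timer; focus events are stubs.
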(event Custom|DisplayUI
  (bind _entryref (Variables|Default|GetEntryRef)
    (:then
      (Variables|/Game/Blueprints/UI/NewEntry_WID.NewEntry_WID_C|SetTimer _entryref 0.0))
    (:else
      (bind _returnvalue (UserInterface|CreateWidget "/Game/Blueprints/UI/NewEntry_WID.NewEntry_WID_C" (Game|GetPlayerController 0) 0))
      (bind _output_get (Variables|Default|SetEntryRef _returnvalue))
      (UserInterface|Viewport|AddtoViewport _output_get 0))))

(event Custom|VFX_OnInteract
  (bind _fx_interactable (Variables|Default|GetFX_Interactable))
  ;[0.2958 0.6571 1] VFX
  (if (Variables|SparkleVFX|GetKillOnGet)
    ;;[1 1 1] Stop Spawning Particles
    (Niagara|SetNiagaraVariable(Float) _fx_interactable "SpawnRate" 0.0)
    (Niagara|SetNiagaraVariable(Float) _fx_interactable "Brightness" (* (Variables|SparkleVFX|GetParticleBrightness) 2.0))
    (else
      (bind _colorlerp (Timeline|VFX_Interact_Color_Change PlayFromStart)
        (:Update
          (Niagara|SetNiagaraVariable(LinearColor) (Variables|Default|GetFX_Interactable) "GlowColor" (Math|Color|Lerp(LinearColor) (Variables|SparkleVFX|GetParticleColor) (Variables|SparkleVFX|GetPushInteractColor) _colorlerp)))))))

(event EventBeginPlay
  (bind _fx_interactable (Variables|Default|GetFX_Interactable))
  ;[0.2958 0.6571 1] VFX
  ;;[1 1 1] Send Static Mesh To Niagara Component
  (Class|NiagaraFunctionLibrary|OverrideSystemUserVariableStaticMeshComponent _fx_interactable "InteractableMesh" (Variables|Default|GetMesh))
  (Niagara|SetNiagaraVariable(LinearColor) _fx_interactable "GlowColor" (Variables|SparkleVFX|GetParticleColor))
  (Niagara|SetNiagaraVariable(Float) _fx_interactable "Brightness" (Variables|SparkleVFX|GetParticleBrightness))
  (Niagara|SetNiagaraVariable(Float) _fx_interactable "SpawnRate" (Variables|SparkleVFX|GetNumberOfParticles))
  (Niagara|SetNiagaraVariable(Float) _fx_interactable "ParticleOffset" (Variables|SparkleVFX|GetParticleNormalOffset)))

(event Collision|EventActorBeginOverlap
  (params (OtherActor :type Actor%20Object%20Reference)))

(event EventTick
  (params (DeltaSeconds :type Float%20%28single-precision%29)))

(event EventOnFocus
  (if (Variables|Default|GetIsInteractable)
    _))

(event EventOnInteract
  (if (Variables|Default|GetIsInteractable)
    (bind _asfirst_person_character (Utilities|Casting|CastToFirstPersonCharacter (Game|GetPlayerCharacter 0)))
    (Default|UnlockJournalEntry (Variables|/Game/Blueprints/FirstPersonCharacter.FirstPersonCharacter_C|GetGrimoireComponent _asfirst_person_character) (Variables|Default|GetObjectID))
    (Variables|Default|SetIsInteractable false)
    (CallFunction|VFXonInteract)))

(event EventLookAway
  (if (Variables|Default|GetIsInteractable)
    _))

(fn ConstructionScript)

(fn GetInteractable
  (return (Variables|Default|GetIsInteractable)))