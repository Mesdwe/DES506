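; Genhu, a giant AI companion character that trails the player and performs spell actions in the world.
; A looping timer and delayed self-call re-issue AIMoveTo when the player is far, and tasks pause following through a flag.
; Spells move it to locations (teleporting on partial paths), purify water using limited, resettable power, and operate BP_GLH in timed stages.
; Pushing interacts with the first interface-implementing actor in a debug-drawn foot-level sphere overlap.
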(event Custom|Follow%20Player
  (if (Variables|Default|GetFollowPlayer?)
    (if (>= (Transformation|GetDistanceTo (Variables|Default|GetChar%20REF)) 1.5e+03)
      (AI|AIMoveTo self "0, 0, 0" (Variables|Default|GetChar%20REF) 2e+02 false
        (:then
          _)))
    (Utilities|FlowControl|Delay 0.2)
    (CallFunction|FollowPlayer)))

(event EventBeginPlay
  (bind _asfirst_person_character (Utilities|Casting|CastToFirstPersonCharacter (Game|GetPlayerCharacter 0)))
  (Variables|Default|SetChar%20Ref _asfirst_person_character)
  (CallFunction|FollowPlayer)
  (Utilities|Time|SetTimerbyEvent (delegate Custom|Follow%20Player) 1.0 true))

(event EventMoveGenhuto
  (params (Location :type Vector :default "0, 0, 0"))
  (bind _returnvalue (Pawn|GetController))
  (bind (_x _y) (Math|Vector|BreakVector Location))
  ;[1 1 1] Move Giant
  (Utilities|Casting|CastToGenhu_Controller _returnvalue)
  (AI|AIMoveTo _returnvalue 0 Location 0 0.0 false
    (:then
      (if (Class|AIController|HasPartialPath (AI|GetAIController self))
        (Transformation|SetActorLocation (Math|Vector|MakeVector _x _y 6e+02) false false)
        (Class|NavMovementComponent|StopActiveMovement (Variables|Character|GetCharacterMovement))))))

(event EventPurifyWater
  (params (WaterRef :type Water%201%20Blueprint%20Object%20Reference))
  ;[1 1 1] Purify Water
  (Utilities|IsValid WaterRef
    (:Is%20Valid
      (bind _waterstatus (Default|CheckWater WaterRef))
      (if _waterstatus
        (Development|PrintString "PureWater")
        (else
          ;;[1 1 1] Stop Follow
          (Variables|Default|SetFollowPlayer? false)
          (AI|AIMoveTo self "0, 0, 0" WaterRef 3e+01 false
            (:OnSuccess
              (Variables|Default|SetIsPurifyingWater? true)
              ;;[1 1 1] Check for purify power
              (if (> (Variables|Default|GetPurifyPower) 0)
                (Default|Purify1 WaterRef)
                (Utilities|FlowControl|Delay 4.0)
                (Utilities|Time|SetTimerbyFunctionName 0 "Purify Water" 0.0)
                (Variables|Default|SetPurifyPower (- (Variables|Default|GetPurifyPower) 1))
                ;;[1 1 1] Start Follow after purify
                (Variables|Default|SetFollowPlayer? true)
                (Variables|Default|SetIsPurifyingWater? false)
                (else
                  (Development|PrintString "PromptForPurifySelf" true true "(R=0.046875,G=1.000000,B=0.141052,A=1.000000)")
                  (Variables|Default|SetFollowPlayer? true))))
            (:OnFail
              (Development|PrintString "Fail to move" true true "(R=1.000000,G=0.000000,B=0.000000,A=1.000000)"))))))))

(event EventPurifySelf
  ;[1 1 1] Purify Genhu
  (Variables|Default|SetIsPurifyingGenhu? true)
  (Variables|Default|SetPurifyPower 2)
  (Development|PrintString "ResetGenhu")
  (Utilities|FlowControl|Delay 2.0)
  (Variables|Default|SetIsPurifyingGenhu? false))

(event EventPushing
  ;[1 1 1] Push Object
  (bind _outactors (CallFunction|SphereOverlapActors (- (Transformation|GetActorLocation) (Math|Vector|MakeVector 0.0 0.0 (Components|Capsule|GetScaledCapsuleHalfHeight (Variables|Collision|GetCapsuleComponent)))) (Variables|/Game/Blueprints/TestAI/PushComponent.PushComponent_C|GetPushRange (Variables|Default|GetPushComponent))))
  (bind _array_element (Utilities|Array|ForEachLoopwithBreak _outactors :!label _label)
    (:LoopBody
      (if (Utilities|DoesObjectImplementInterface _array_element "/Game/Blueprints/TestAI/BP_InteractInterface.BP_InteractInterface_C")
        (Class|BPInteractInterface|OnInteracted(Message) _array_element self)
        (goto _label Break)))))

(event EventSpellError
  ;[1 1 1] Spell Error
  (Variables|Default|SetIsError? true)
  (Utilities|FlowControl|Delay 2.0)
  (Variables|Default|SetIsError? false))

(event EventGLH
  (bind _returnvalue (Actor|GetActorOfClass "/Game/Blueprints/TestAI/BP_GLH.BP_GLH_C"))
  (Utilities|IsValid _returnvalue
    (:Is%20Valid
      (Variables|Default|SetFollowPlayer? false)
      (AI|AIMoveTo self (Math|Vector|MakeVector (.x (+ (Transformation|GetActorLocation _returnvalue) "-270.000000,290.000000,0.000000")) (.y (+ (Transformation|GetActorLocation _returnvalue) "-270.000000,290.000000,0.000000")) 0.0) 0 5.0 false
        (:OnSuccess
          (Variables|Default|SetLiftNum (+ (Variables|Default|GetLiftNum) 1))
          (Utilities|FlowControl|Delay 4.0)
          (Default|LiftHand _returnvalue)
          (Variables|Default|SetLiftNum (+ (Variables|Default|GetLiftNum) 1))
          (Utilities|FlowControl|Delay 4.0)
          (Default|HandDown _returnvalue)
          (Variables|Default|SetLiftNum (+ (Variables|Default|GetLiftNum) 1))
          (Utilities|FlowControl|Delay 0.5)
          (Variables|Default|SetFollowPlayer? true)
          (Variables|Default|SetLiftNum 0))
        (:OnFail
          (Development|PrintString "Fail to Move"))))
    (:Is%20Not%20Valid
      (Development|PrintString "Lift not Valid"))))

(fn ConstructionScript)

(fn SphereOverlapActors
  (params (Center :type Vector) (Radius :type Float%20%28single-precision%29))
  (Utilities|FlowControl|Sequence
    (:then_0
      (Rendering|Debug|DrawDebugSphere Center Radius 12 "(R=1.000000,G=1.000000,B=1.000000,A=1.000000)" 2.0 1.0))
    (:then_1
      (bind _outactors (Collision|SphereOverlapActors Center Radius (Utilities|Array|MakeArray "ObjectTypeQuery2") 0 (Utilities|Array|MakeArray self)))
      (return _outactors))))