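; SpellComponentBP manages the player's rune-based spell casting menu.
; Activate and deactivate events call the matching casting calls, then create or remove the CastingMenu widget.
; Four rune events forward their number as a string to the open menu's GetRuneInput.
; An invalid spell prints a debug message and triggers SpellError on the first-person character's GenhuRef.
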(event Custom|ShowCastingMenu
  (Variables|Default|GetCastingMenu
    (:then)
    (:else
      (bind _returnvalue (UserInterface|CreateWidget "/Game/Blueprints/UI/CastingMenu_WID.CastingMenu_WID_C" (Game|GetPlayerController 0)))
      (bind _output_get (Variables|Default|SetCastingMenu _returnvalue))
      (UserInterface|Viewport|AddtoViewport _output_get 0))))

(event Custom|HideCastingMenu
  (Variables|Default|GetCastingMenu
    (:then
      (Widget|RemovefromParent (Variables|Default|GetCastingMenu))
      (Variables|Default|SetCastingMenu 0))
    (:else)))

(event EventOnActivateCastingMenu
  (Default|CallActivateCasting)
  (CallFunction|ShowCastingMenu))

(event EventOnDeactivateCastingMenu
  (Default|CallDeactivateCasting)
  (CallFunction|HideCastingMenu))

(event EventInvalidSpell
  (Development|PrintString "Invalid")
  (bind _asfirst_person_character (Utilities|Casting|CastToFirstPersonCharacter (Game|GetPlayerCharacter 0)))
  (Default|SpellError (Variables|/Game/Blueprints/FirstPersonCharacter.FirstPersonCharacter_C|GetGenhuRef _asfirst_person_character)))

(event EventRune1Behaviour
  (bind _castingmenu (Variables|Default|GetCastingMenu)
    (:then
      (Default|GetRuneInput _castingmenu "1"))
    (:else)))

(event EventRune2Behaviour
  (bind _castingmenu (Variables|Default|GetCastingMenu)
    (:then
      (Default|GetRuneInput _castingmenu "2"))
    (:else)))

(event EventRune3Behaviour
  (bind _castingmenu (Variables|Default|GetCastingMenu)
    (:then
      (Default|GetRuneInput _castingmenu "3"))
    (:else)))

(event EventRune4Behaviour
  (bind _castingmenu (Variables|Default|GetCastingMenu)
    (:then
      (Default|GetRuneInput _castingmenu "4"))
    (:else)))