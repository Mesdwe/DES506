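; Pushable object that the giant Genhu pushes until its mesh overlaps a BP_EndPush, then reveals Mesh2 and destroys itself.
; On interaction it polls until Genhu nears a push transform and the player clears it, then snaps Genhu there and starts its PushComponent.
; The closest-transform search effectively returns the last index, and placement trace checks are bypassed.
; Construction draws arrows at push transforms; Tick eases emissive and light toward VFX targets.
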(event OnComponentBeginOverlap(Mesh)
  (params (OverlappedComponent :type Primitive%20Component%20Object%20Reference) (OtherActor :type Actor%20Object%20Reference) (OtherComp :type Primitive%20Component%20Object%20Reference) (OtherBodyIndex :type Integer) (bFromSweep :type Boolean) (SweepResult :type Hit%20Result%20Structure%20%28by%20ref%29))
  (bind _mesh2 (Variables|Default|GetMesh2))
  (Utilities|Casting|CastToBP_EndPush OtherActor)
  (bind _asfirst_person_character (Utilities|Casting|CastToFirstPersonCharacter (Game|GetPlayerCharacter 0)))
  (Default|EndPush (Variables|/Game/Blueprints/Genhu_Character.Genhu_Character_C|GetPushComponent (Variables|/Game/Blueprints/FirstPersonCharacter.FirstPersonCharacter_C|GetGenhuRef _asfirst_person_character)))
  (CallFunction|VFXonPushDeactivated)
  (Utilities|IsValid _mesh2
    (:Is%20Valid
      (Rendering|SetVisibility (Variables|/Script/Engine.StaticMeshActor|GetStaticMeshComponent _mesh2) true false)
      (Actor|DestroyActor))))

(event EventBeginPlay)

(event Collision|EventActorBeginOverlap
  (params (OtherActor :type Actor%20Object%20Reference)))

(event EventTick
  (params (DeltaSeconds :type Float%20%28single-precision%29)))

(event EventOnInteracted
  (params (Giant :type Genhu%20Character%20Object%20Reference))
  (bind _pushcomponent (Variables|/Game/Blueprints/Genhu_Character.Genhu_Character_C|GetPushComponent Giant))
  (bind _gateref (Variables|Default|GetGateRef))
  (bind _pushrange (Variables|/Game/Blueprints/TestAI/PushComponent.PushComponent_C|GetPushRange _pushcomponent))
  (bind _bestindex (CallFunction|FindClosestPushTransformIndex (Math|Conversions|ToVector2D(Vector) (Transformation|GetActorLocation Giant)) _pushrange))
  ;[1 1 1] Wait for Genhu walk to push range
  (if (<= (Math|Vector|Distance2D(Vector) (Math|Conversions|ToVector2D(Vector) (Math|Transform|TransformLocation (Transformation|GetActorTransform) (.location (Utilities|Array|Get(acopy) (Variables|Default|GetPushTransforms) _bestindex)))) (Math|Conversions|ToVector2D(Vector) (Transformation|GetActorLocation Giant))) _pushrange) :!label _label
    ;[1 1 1] Wait for player leave space for push
    (if (> (Math|Vector|Distance2D(Vector) (Math|Conversions|ToVector2D(Vector) (Math|Transform|TransformLocation (Transformation|GetActorTransform) (.location (Utilities|Array|Get(acopy) (Variables|Default|GetPushTransforms) _bestindex)))) (Math|Conversions|ToVector2D(Vector) (Transformation|GetActorLocation (Game|GetPlayerCharacter 0)))) 2e+02) :!label _label_2
      (CallFunction|HandleInteraction Giant _bestindex)
      (Variables|Default|SetIsPushed? true)
      ;[0.2033 1 0.4447] Trigger VFX push
      (Utilities|IsValid _gateref
        (:Is%20Valid
          (Default|VFXPushDebris _gateref)
          (CallFunction|VFXonGenhuPush)))
      (else
        (Utilities|FlowControl|Delay 0.4)
        (goto _label_2)))
    (else
      (Utilities|FlowControl|Delay 0.6)
      (goto _label))))

(event Custom|VFX_OnPushDeactivated
  (Variables|Default|SetTargetEmissive 0.0)
  (Variables|Default|SetTargetLightIntensity 0.0))

(event Custom|VFX_OnPushActivated
  (Variables|Default|SetTargetEmissive 1.8)
  (Variables|Default|SetTargetLightIntensity 3.5e+04))

(event Custom|VFX_OnGenhuPush
  (Niagara|SetNiagaraVariable(Float) (Variables|Default|GetFX_Interactable) "SpawnRate" 0.0))

(event EventTick
  (params (DeltaSeconds :type Float%20%28single-precision%29))
  (bind _targetemissive (Variables|Default|GetTargetEmissive))
  ;[1 1 1] Gradually adjust emissive to target
  (if (!= _targetemissive (Variables|Default|GetCurrentEmissive))
    (bind _output_get (Variables|Default|SetCurrentEmissive (Math|Float|Lerp (Variables|Default|GetCurrentEmissive) _targetemissive 0.1)))
    (Rendering|Material|SetScalarParameterValueonMaterials (Variables|Character|GetMesh) "Emissive Multiplier" _output_get)
    ;[1 1 1] Gradually adjust point light to target
    (bind _output_get_2 (Variables|Default|SetCurrentLightIntensity (Math|Float|Lerp (Variables|Default|GetCurrentLightIntensity) (Variables|Default|GetTargetLightIntensity) 0.1)))
    (Rendering|Components|Light|SetIntensity (Variables|Default|GetPointLight) _output_get_2)))

(fn ConstructionScript
  (for _array_element (Variables|Default|GetPushTransforms)
    (AddComponent|AddArrowComponent false _array_element)))

(fn HandleInteraction
  (params (Character :type Character%20Object%20Reference) (BestIndex :type Integer))
  (bind _returnvalue (Transformation|GetActorTransform))
  (bind _pushtransforms (Variables|Default|GetPushTransforms))
  (bind _output (Utilities|Array|Get(acopy) _pushtransforms BestIndex))
  (bind _capsulecomponent (Variables|/Script/Engine.Character|GetCapsuleComponent Character))
  (bind _returnvalue_2 (Math|Transform|ComposeTransforms _output _returnvalue))
  (Utilities|IsValid Character
    (:Is%20Valid
      (bind _output_get (LocalVariables|SetPush%20Component (Actor|GetComponentbyClass Character "/Game/Blueprints/TestAI/PushComponent.PushComponent_C")))
      (Utilities|IsValid _output_get
        (:Is%20Valid
          (if (>= BestIndex 0)
            (bind _output_get_2 (LocalVariables|SetCharacterNewTransform (Math|Transform|MakeTransform (.location _returnvalue_2) (.rotation _returnvalue_2) (.scale _returnvalue_2))))
            (bind _outhit (Collision|CapsuleTraceByChannel (+ (.location (LocalVariables|GetCharacterNewTransform)) "0, 0,70.000000") (- (.location (LocalVariables|GetCharacterNewTransform)) "0, 0,100.000000") (Components|Capsule|GetScaledCapsuleRadius _capsulecomponent) (Components|Capsule|GetScaledCapsuleHalfHeight _capsulecomponent) "TraceTypeQuery1" false 0 "None" true "(R=1.000000,G=0.000000,B=0.000000,A=1.000000)" "(R=0.000000,G=1.000000,B=0.000000,A=1.000000)" 2.0))
            (if true
              (if true
                (bind (_outhit_2 _returnvalue_3) (Collision|LineTraceByChannel (Transformation|GetActorLocation) (.location (LocalVariables|GetCharacterNewTransform)) "TraceTypeQuery1" false (Utilities|Array|MakeArray Character) "None" true "(R=1.000000,G=0.000000,B=0.000000,A=1.000000)" "(R=0.000000,G=1.000000,B=0.000000,A=1.000000)" 2.0))
                (if true
                  (Transformation|SetActorTransform Character (Math|Transform|MakeTransform (.location (LocalVariables|GetCharacterNewTransform)) (.rotation (LocalVariables|GetCharacterNewTransform)) "1,1,1") false true)
                  (Default|BeginPush (LocalVariables|GetPush%20Component) self)
                  (else
                    (Utilities|PushFailedInfo "Wall between Genhu and object")))
                (else
                  (Utilities|PushFailedInfo "Floor not walkable")))
              (else
                (Utilities|PushFailedInfo "No room stand")))
            (else
              (Utilities|PushFailedInfo "No push transform found"))))
        (:Is%20Not%20Valid
          (Utilities|PushFailedInfo "Character does not have push component"))))
    (:Is%20Not%20Valid
      (Utilities|PushFailedInfo "Character is invaild"))))

(fn FindClosestPushTransformIndex
  (params (CharacterLocation :type Vector%202D%20Structure) (PushRange :type Float%20%28single-precision%29))
  (for (_array_element _array_index) (Variables|Default|GetPushTransforms)
    (LocalVariables|SetCurrentTransformIndex _array_index)
    (bind _output_get (LocalVariables|SetCurrentDistanceSq (Class|KismetMathLibrary|DistanceSquared2D (Math|Conversions|ToVector2D(Vector) (Math|Transform|TransformLocation (Transformation|GetActorTransform) (.location _array_element))) CharacterLocation)))
    (if (< _output_get (Math|Float|Square PushRange))
      (if (or (< (LocalVariables|GetCurrentDistanceSq) (LocalVariables|GetCloestDistanceSq)) (< (LocalVariables|GetCloestTransformIndex) 0))
        (LocalVariables|SetCloestTransformIndex (LocalVariables|GetCloestTransformIndex))
        (LocalVariables|SetCloestDistanceSq (LocalVariables|GetCloestDistanceSq)))))
  (return (LocalVariables|GetCurrentTransformIndex)))