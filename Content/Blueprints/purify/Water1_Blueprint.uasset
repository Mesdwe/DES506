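; Water source actor that starts as sludge and turns clean when PurifyWater is triggered, exposing its status through CheckWater.
; PurifyWater plays a timeline that drives the Sludginess material parameter and sets the status, while Niagara area-of-effect particles, using the PurifyRangeBall mesh as their volume, spawn until the transition finishes.
; After a delay, it finds all BP_SludgeWall actors and dissolves those within PurifyRange.
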(event Custom|PurifyWater
  (Utilities|FlowControl|Sequence
    (:then_0
      ;[1 1 1] Spawn AoE Paricles
      (Niagara|SetNiagaraVariable(Float) (Variables|Default|GetFX_AoE_Purification) "Spawn_Rate" 1e+02)
      ;[1 1 1] Material Transition
      (bind _sludginess (Timeline|Timeline_0 Play)
        (:Update
          (bind _output_get (Variables|MaterialParameters|SetSludginess _sludginess))
          (Rendering|Material|SetScalarParameterValueonMaterials (Variables|Debug|GetStaticMeshComponent) "Sludginess" _output_get)
          (Variables|Default|SetWaterStatus true))
        (:Finished
          ;[1 1 1] Disable AoE Particles
          (Niagara|SetNiagaraVariable(Float) (Variables|Default|GetFX_AoE_Purification) "Spawn_Rate" 0.0)
          (Class|NiagaraComponent|SetRenderingEnabled (Variables|Default|GetFX_AoE_Purification) false))))
    (:then_2
      ;[1 1 1] DestroySludgeWall
      (Utilities|FlowControl|Delay 4.0)
      (bind _outactors (Actor|GetAllActorsOfClass "/Game/Blueprints/purify/BP_SludgeWall.BP_SludgeWall_C"))
      (bind _array_element (Utilities|Array|ForEachLoopwithBreak _outactors)
        (:LoopBody
          (if (<= (Transformation|GetDistanceTo _array_element self) (Variables|Default|GetPurifyRange))
            (Utilities|IsValid _array_element
              (:Is%20Valid
                (Default|WallDissolve _array_element)))))))))

(event EventBeginPlay
  (Utilities|FlowControl|Sequence
    (:then_0
      ;[1 1 1] Set Material to sludge
      (Rendering|Material|SetScalarParameterValueonMaterials (Variables|Debug|GetStaticMeshComponent) "Sludginess" (Variables|MaterialParameters|GetSludginess)))
    (:then_1
      ;[1 1 1] Set Up Area of Effect VFX
      (Class|NiagaraFunctionLibrary|OverrideSystemUserVariableStaticMeshComponent (Variables|Default|GetFX_AoE_Purification) "Mesh_Volume" (Variables|Default|GetPurifyRangeBall))
      (Niagara|SetNiagaraVariable(Float) (Variables|Default|GetFX_AoE_Purification) "Spawn_Rate" 0.0))))

(event Collision|EventActorBeginOverlap
  (params (OtherActor :type Actor%20Object%20Reference)))

(event EventTick
  (params (DeltaSeconds :type Float%20%28single-precision%29)))

(fn ConstructionScript
  (bind _returnvalue (Rendering|Material|CreateDynamicMaterialInstance (Variables|Debug|GetStaticMeshComponent) 0 "/Game/Art/VFX/Water-Sludge/M_WaterSource_Inst.M_WaterSource_Inst" "None" :!class /Script/Engine.PrimitiveComponent))
  (Variables|Default|SetSludgeMeterialRef _returnvalue))

(fn CheckWater
  (return (Variables|Default|GetWaterStatus)))