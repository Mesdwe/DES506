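; Environmental VFX actor that starts Niagara rain over the first-person character once they enter a trigger.
; Each tick while raining, it moves the rain spawn point just above the player and updates the Niagara spawn rate.
; The rate is a clamped lerp on the spawn point's distance from the trigger, so rain grows heavier as the player moves away.
; Nothing turns the rain off after activation.
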(event OnComponentBeginOverlap(Rain_Trigger)
  (params (OverlappedComponent :type Primitive%20Component%20Object%20Reference) (OtherActor :type Actor%20Object%20Reference) (OtherComp :type Primitive%20Component%20Object%20Reference) (OtherBodyIndex :type Integer) (bFromSweep :type Boolean) (SweepResult :type Hit%20Result%20Structure%20%28by%20ref%29))
  ;[1 1 1] Begin rain if player enters rain_trigger
  (if (== OtherActor (Variables|Default|GetPlayer_Ref))
    (CallFunction|ActivateRain)))

(event Custom|ActivateRain
  (Variables|Default|SetisRaining true))

(event Custom|DeactivateRain
  (Niagara|SetNiagaraVariable(Float) (Variables|Default|GetNiagara-Rain) "Spawn_Rate" (Variables|Default|GetRainRate))
  (Variables|Default|SetisRaining false))

(event EventBeginPlay
  ;[1 1 1] Get Reference to Player Location
  (bind _returnvalue (Actor|GetActorOfClass "/Game/Blueprints/FirstPersonCharacter.FirstPersonCharacter_C"))
  (Utilities|IsValid _returnvalue
    (:Is%20Valid
      (Variables|Default|SetPlayer_Ref _returnvalue)
      (CallFunction|DeactivateRain))))

(event EventTick
  (params (DeltaSeconds :type Float%20%28single-precision%29))
  (if (Variables|Default|GetisRaining)
    ;[1 1 1] Set rain emitted to players location
    (Transformation|SetWorldLocation (Variables|Default|GetRain-Spawn) (+ (.location (Transformation|GetActorTransform (Variables|Default|GetPlayer_Ref))) "0, 0,100.000000") false false)
    (Variables|Default|SetRainRate (Math|Float|Lerp 0.0 5e+02 (Math|Float|Clamp(Float) (/ (Math|Vector|Distance(Vector) (Transformation|GetWorldLocation (Variables|Default|GetRain-Spawn)) (Transformation|GetWorldLocation (Variables|Default|GetRain_Trigger))) 1e+04))))
    (Niagara|SetNiagaraVariable(Float) (Variables|Default|GetNiagara-Rain) "Spawn_Rate" (Variables|Default|GetRainRate))))

(fn ConstructionScript)