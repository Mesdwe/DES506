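; BP_BlackRain_EndSequence is an environmental VFX actor that switches a Niagara rain effect between two intensities, named for the end sequence.
; On BeginPlay it caches the FirstPersonCharacter and, if found, starts in the deactivated state.
; ActivateRain and DeactivateRain set the Niagara Spawn_Rate variable to RainRateMaximum or RainRate respectively and update the IsRaining flag.
; The stored player reference is not used elsewhere in this graph.
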(event Custom|ActivateRain
  (Variables|Default|SetisRaining true)
  (Niagara|SetNiagaraVariable(Float) (Variables|Default|GetNiagara-Rain) "Spawn_Rate" (Variables|Default|GetRainRate_Maximum)))

(event Custom|DeactivateRain
  (Niagara|SetNiagaraVariable(Float) (Variables|Default|GetNiagara-Rain) "Spawn_Rate" (Variables|Default|GetRainRate))
  (Variables|Default|SetisRaining false))

(event EventBeginPlay
  ;[1 1 1] Get Reference to Player Location
  (bind _returnvalue (Actor|GetActorOfClass "/Game/Blueprints/FirstPersonCharacter.FirstPersonCharacter_C"))
  (Utilities|IsValid _returnvalue
    (:Is%20Valid
      (Variables|Default|SetPlayer_Ref _returnvalue)
      (CallFunction|DeactivateRain))))

(fn ConstructionScript)