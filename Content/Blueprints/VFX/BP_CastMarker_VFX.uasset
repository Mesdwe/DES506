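; Cast marker VFX that shows whether the current cast is valid through a dust cloud and an intersection cylinder.
; The construction script creates a dynamic material instance for the cylinder.
; Tick watches CastIsValid: when invalid it whitens the dust at a target opacity and desaturates and fades the cylinder, and when valid again it restores defaults.
; A DustGreyedOut flag ensures parameters change only on transitions; BeginPlay applies the default look.
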(event EventBeginPlay
  ;[1 1 1] Return to default material values
  (Effects|Components|ParticleSystem|SetColorParameter (Variables|Default|GetDustCloud) "DustColor" (Math|Conversions|ToLinearColor(Color) (Variables|DustFX|GetDustColor)))
  (Rendering|Material|SetScalarParameterValue (Variables|Cylinder|GetMaterial_Inst) "OpacityMultiplier" 1.0 :!class /Script/Engine.MaterialInstanceDynamic)
  (Rendering|Material|SetScalarParameterValue (Variables|Cylinder|GetMaterial_Inst) "Saturation" 1.0 :!class /Script/Engine.MaterialInstanceDynamic)
  (Variables|GreyOut|SetDustGreyedOut false))

(event EventTick
  (params (DeltaSeconds :type Float%20%28single-precision%29))
  (bind _returnvalue (Class|KismetMathLibrary|LinearColorWhite))
  (bind _returnvalue_2 (Math|Conversions|ToColor(LinearColor) _returnvalue))
  (bind (_b _g _r) (Math|Color|BreakColor _returnvalue_2))
  ;[1 1 1] Check if cast is valid and greyed out
  (if (Variables|Components|GetcastIsValid)
    (if (Variables|GreyOut|GetDustGreyedOut)
      ;[1 1 1] Return to default material values
      (Effects|Components|ParticleSystem|SetColorParameter (Variables|Default|GetDustCloud) "DustColor" (Math|Conversions|ToLinearColor(Color) (Variables|DustFX|GetDustColor)))
      (Rendering|Material|SetScalarParameterValue (Variables|Cylinder|GetMaterial_Inst) "OpacityMultiplier" 1.0 :!class /Script/Engine.MaterialInstanceDynamic)
      (Rendering|Material|SetScalarParameterValue (Variables|Cylinder|GetMaterial_Inst) "Saturation" 1.0 :!class /Script/Engine.MaterialInstanceDynamic)
      (Variables|GreyOut|SetDustGreyedOut false))
    (elif (not (Variables|GreyOut|GetDustGreyedOut))
      ;[1 1 1] Grey-out Cast Dust
      (Effects|Components|ParticleSystem|SetColorParameter (Variables|Default|GetDustCloud) "DustColor" (Math|Conversions|ToLinearColor(Color) (Math|Color|MakeColor _b _g _r (Variables|GreyOut|GetTargetDustOpacity))))
      (Rendering|Material|SetScalarParameterValue (Variables|Cylinder|GetMaterial_Inst) "OpacityMultiplier" (/ (Variables|GreyOut|GetTargetCylinderOpacity) 255.0) :!class /Script/Engine.MaterialInstanceDynamic)
      (Rendering|Material|SetScalarParameterValue (Variables|Cylinder|GetMaterial_Inst) "Saturation" 0.0 :!class /Script/Engine.MaterialInstanceDynamic)
      (Variables|GreyOut|SetDustGreyedOut true))))

(fn ConstructionScript
  (bind _returnvalue (Rendering|Material|CreateDynamicMaterialInstance (Variables|Default|GetIntersectCylinder) 0 0 "None" :!class /Script/Engine.PrimitiveComponent))
  (Variables|Cylinder|SetMaterial_Inst _returnvalue))