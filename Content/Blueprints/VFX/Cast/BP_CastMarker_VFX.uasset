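; Cast marker VFX actor that shows the current spell type (Move, Purify, Push or Invalid) through color, spin speed and particles.
; SetCastType sets a target color and rotation rate, after a short delay for valid spells; only Move activates its own effect, while Invalid deactivates all three.
; While the color differs from its target, Tick lerps color and rotation into the mesh's dynamic material and recolors the point light.
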(event Custom|SetCastType
  (params (Spell :type Name))
  (if (Utilities|Name|NotEqual(Name) (Variables|Default|GetSpell) Spell)
    (if (or (Utilities|Name|NotEqual(Name) Spell "Invalid") (Utilities|Name|NotEqual(Name) (Variables|Default|GetSpell) "Invalid"))
      _
      (else
        (Components|Activation|Activate (Variables|Default|GetFX_SpawnFeedback) false)))
    (bind _output_get (Variables|Default|SetSpell Spell))
    (switch name _output_get
      (:Move
        ;[0.1253 0.215 0.3125] Move Cast
        (Utilities|FlowControl|Delay 0.2)
        (Variables|Default|SetTargetColor (Variables|Default|GetMoveColor))
        (Variables|Default|SetTargetRotationRate 3.0)
        (Components|Activation|Activate (Variables|Default|GetFX_Move) true))
      (:Purify
        ;[0.2346 0.05649 0.3125] Purify
        (Utilities|FlowControl|Delay 0.2)
        (Variables|Default|SetTargetColor (Variables|Default|GetPurifyColor))
        (Variables|Default|SetTargetRotationRate 3.0))
      (:Push
        ;[0.8385 0.6557 0.08735] Push
        (Utilities|FlowControl|Delay 0.2)
        (Variables|Default|SetTargetColor (Variables|Default|GetPushColor))
        (Variables|Default|SetTargetRotationRate 3.0))
      (:Invalid
        ;[1 0 0.01504] Invalid Cast
        (Variables|Default|SetTargetColor (Variables|Default|GetInvalidColor))
        (Variables|Default|SetTargetRotationRate 1.0)
        (Components|Activation|Deactivate (Variables|Default|GetFX_Move))
        (Components|Activation|Deactivate (Variables|Default|GetFX_Purify))
        (Components|Activation|Deactivate (Variables|Default|GetFX_Push))))))

(event EventBeginPlay
  (bind _currentcolor (Variables|Default|GetCurrentColor))
  (bind _material_inst (Variables|Cylinder|GetMaterial_Inst))
  ;[1 1 1] Set Up
  (Rendering|Material|SetVectorParameterValue _material_inst "Emmisive" _currentcolor :!class /Script/Engine.MaterialInstanceDynamic)
  (Rendering|Material|SetScalarParameterValue _material_inst "Opacity" (.A (Math|Color|BreakColor _currentcolor)) :!class /Script/Engine.MaterialInstanceDynamic)
  (Rendering|Components|Light|SetLightColor (Variables|Default|GetPointLight) "(R=0.000000,G=0.000000,B=0.000000,A=1.000000)" true))

(event EventTick
  (params (DeltaSeconds :type Float%20%28single-precision%29))
  ;[1 1 1] Update Color
  (Utilities|FlowControl|Sequence
    (:then_0
      (if (!= (Variables|Default|GetCurrentColor) (Variables|Default|GetTargetColor))
        (bind _output_get (Variables|Default|SetCurrentColor (Math|Color|Lerp(LinearColor) (Variables|Default|GetCurrentColor) (Variables|Default|GetTargetColor) 0.2)))
        (Rendering|Material|SetVectorParameterValue (Variables|Cylinder|GetMaterial_Inst) "EmissiveColor" _output_get :!class /Script/Engine.MaterialInstanceDynamic)
        (Rendering|Components|Light|SetLightColor (Variables|Default|GetPointLight) _output_get true)
        (Rendering|Material|SetScalarParameterValue (Variables|Cylinder|GetMaterial_Inst) "Opacity" (.A (Math|Color|BreakColor (Math|Color|Lerp(LinearColor) (Variables|Default|GetCurrentColor) (Variables|Default|GetTargetColor) 0.2))) :!class /Script/Engine.MaterialInstanceDynamic)
        (bind _output_get_2 (Variables|Default|SetCastRotationRate (Math|Float|Lerp (Variables|Default|GetCastRotationRate) (Variables|Default|GetTargetRotationRate) 0.2)))
        (Rendering|Material|SetScalarParameterValue (Variables|Cylinder|GetMaterial_Inst) "RotationSpeed" _output_get_2 :!class /Script/Engine.MaterialInstanceDynamic)))))

(fn ConstructionScript
  (bind _returnvalue (Rendering|Material|CreateDynamicMaterialInstance (Variables|Default|GetSM_Cast) 0 0 "None" :!class /Script/Engine.PrimitiveComponent))
  (Variables|Cylinder|SetMaterial_Inst _returnvalue))