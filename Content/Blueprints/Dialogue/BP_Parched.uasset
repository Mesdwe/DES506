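; BP_Parched is an interactable dialogue actor that groans and shows a random quip when the player interacts with it.
; Focus caches the player's DialogueComponent and looking away clears it; interacting restarts the Wwise groan and displays the quip through that component.
; Fetching a quip also unlocks a Grimoire journal entry as a side effect.
; InitDialogue is empty, leaving its mood-filtered data table loading disconnected.
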(event EventOnInteract
  (bind _self self)
  (Class|AkGameplayStatics|StopActor _self)
  (Class|AkGameplayStatics|PostEvent "/Game/Audio/SFX/TheParched/sfx_Parched_Groan.sfx_Parched_Groan" _self)
  (bind _text (CallFunction|GetRandomDialogueQuip))
  (bind _dialogue_component (Variables|Default|GetDialogue%20Component)
    (:then
      (Default|DisplayUI _dialogue_component _text))
    (:else)))

(event EventOnFocus
  (bind _asfirst_person_character (Utilities|Casting|CastToFirstPersonCharacter (Game|GetPlayerCharacter 0)))
  (Variables|Default|SetDialogue%20Component (Variables|/Game/Blueprints/FirstPersonCharacter.FirstPersonCharacter_C|GetDialogueComponent _asfirst_person_character)))

(event EventLookAway
  (Variables|Default|SetDialogue%20Component 0))

(fn ConstructionScript)

(fn GetRandomDialogueQuip
  (bind _asfirst_person_character (Utilities|Casting|CastToFirstPersonCharacter (Game|GetPlayerCharacter 0)))
  (Default|UnlockJournalEntry (Variables|/Game/Blueprints/FirstPersonCharacter.FirstPersonCharacter_C|GetGrimoireComponent _asfirst_person_character) 4)
  (bind _returnvalue (Class|ParchedCharacter|GetRandomQuip))
  (return (Utilities|Text|ToText(String) _returnvalue)))

(fn InitDialogue)

(fn GetInteractable
  (return true))