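; Tuning fork actor whose mesh glows with an emissive cooldown animation when its Strike event fires.
; Strike zeroes the EmissiveIntensity material parameter, then plays the GlowCooldown timeline, which drives it scaled by TargetEmissionStrength.
; BeginPlay runs the same sequence, so the glow also plays at start.
; The construction script stores a dynamic material instance, though glow updates go through the mesh component.
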(event Custom|Strike
  ;[1 1 1] Emissive Cooldown Animation
  (Rendering|Material|SetScalarParameterValueonMaterials (Variables|Default|GetStaticMesh) "EmissiveIntensity" 0.0)
  (bind _emissionintensity (Timeline|GlowCooldown Play)
    (:Update
      (Rendering|Material|SetScalarParameterValueonMaterials (Variables|Default|GetStaticMesh) "EmissiveIntensity" (* _emissionintensity (Variables|Default|GetTargetEmissionStrength))))))

(event EventBeginPlay
  ;[1 1 1] Emissive Cooldown Animation
  (Rendering|Material|SetScalarParameterValueonMaterials (Variables|Default|GetStaticMesh) "EmissiveIntensity" 0.0)
  (bind _emissionintensity (Timeline|GlowCooldown Play)
    (:Update
      (Rendering|Material|SetScalarParameterValueonMaterials (Variables|Default|GetStaticMesh) "EmissiveIntensity" (* _emissionintensity (Variables|Default|GetTargetEmissionStrength))))))

(event Collision|EventActorBeginOverlap
  (params (OtherActor :type Actor%20Object%20Reference)))

(event EventTick
  (params (DeltaSeconds :type Float%20%28single-precision%29)))

(fn ConstructionScript
  (bind _returnvalue (Rendering|Material|CreateDynamicMaterialInstance (Variables|Default|GetStaticMesh) 0 0 "None" :!class /Script/Engine.PrimitiveComponent))
  (Variables|Default|SetTuningForkMaterial _returnvalue))