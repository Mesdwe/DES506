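; Purify Water invocation: a targeting actor that aims a purification cast at water or rivers and unlocks its Grimoire entry on spawn.
; Each tick a camera trace, falling back to a downward trace at max range, snaps it to the surface.
; Hits on Water1_Blueprint or BP_River validate the cast and switch the marker VFX.
; BeginCasting sends purify messages to the player's GenhuRef and destroys the actor when valid.
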(event EventBeginPlay
  (|CallParentFunction)
  (bind _asfirst_person_character (Utilities|Casting|CastToFirstPersonCharacter (Game|GetPlayerCharacter 0)))
  (Variables|Default|SetFirst%20Person%20Camera%20Component (Variables|/Script/Sludge.SludgeCharacter|GetFirstPersonCameraComponent _asfirst_person_character))
  (Default|UnlockInvocationEntry (Variables|/Game/Blueprints/FirstPersonCharacter.FirstPersonCharacter_C|GetGrimoireComponent _asfirst_person_character) "Purify Water" false)
  (bind _asbp_cast_marker_vfx (Utilities|Casting|CastToBP_CastMarker_VFX (Variables|/Script/Engine.ChildActorComponent|GetChildActor (Variables|Default|GetCastMarker))))
  (Variables|Default|SetAs%20BP%20Cast%20Marker%20VFX _asbp_cast_marker_vfx))

(event EventTick
  (params (DeltaSeconds :type Float%20%28single-precision%29))
  (bind _defaultsceneroot (Variables|Default|GetDefaultSceneRoot))
  (bind _first_person_camera_component (Variables|Default|GetFirst%20Person%20Camera%20Component))
  (bind _as_bp_cast_marker_vfx (Variables|Default|GetAs%20BP%20Cast%20Marker%20VFX))
  (bind _as_bp_cast_marker_vfx_2 (Variables|Default|GetAs%20BP%20Cast%20Marker%20VFX))
  (bind _returnvalue (Transformation|GetWorldLocation _first_person_camera_component))
  (bind _returnvalue_2 (Math|Vector|GetForwardVector _first_person_camera_component))
  (bind _returnvalue_3 (Transformation|GetWorldLocation _defaultsceneroot))
  (bind _returnvalue_4 (* _returnvalue_2 1e+03))
  (bind _returnvalue_5 (+ _returnvalue_4 _returnvalue))
  (|CallParentFunction DeltaSeconds)
  (bind (_outhit _returnvalue_6) (Collision|LineTraceByChannel _returnvalue _returnvalue_5 "TraceTypeQuery1" false 0 "None" true "(R=0.021415,G=0.000000,B=1.000000,A=1.000000)"))
  (if _returnvalue_6
    (Transformation|SetActorLocationAndRotation (.Location (Collision|BreakHitResult _outhit)) (Math|Rotator|MakeRotfromZ (.ImpactNormal (Collision|BreakHitResult _outhit))))
    (bind _aswater_1_blueprint (Utilities|Casting|CastToWater1_Blueprint (.HitActor (Collision|BreakHitResult _outhit)))
      (:then
        (Variables|Default|SetNearestWater _aswater_1_blueprint)
        (Variables|Default|SetbHasValidCondition true :!label _label)
        (Default|SetCastType _as_bp_cast_marker_vfx_2 "Purify"))
      (:CastFailed
        (Variables|Default|SetNearestWater 0)
        (bind _asbp_river (Utilities|Casting|CastToBP_River (.HitActor (Collision|BreakHitResult _outhit)))
          (:then
            (Variables|Default|SetAs%20BP%20River _asbp_river)
            (goto _label))
          (:CastFailed
            (Variables|Default|SetAs%20BP%20River 0)
            (Variables|Default|SetbHasValidCondition false)
            (Default|SetCastType _as_bp_cast_marker_vfx_2 "Invalid")))))
    (else
      (Transformation|SetActorLocation _returnvalue_5 false false)
      (bind (_outhit_2 _returnvalue_7) (Collision|LineTraceByChannel _returnvalue_3 (+ _returnvalue_3 (* "0.000000,0.000000,1.000000" -1e+03)) "TraceTypeQuery1" false 0 "None"))
      (if _returnvalue_7
        (Transformation|SetActorLocationAndRotation (.Location (Collision|BreakHitResult _outhit_2)) (Math|Rotator|MakeRotfromZ (.ImpactNormal (Collision|BreakHitResult _outhit_2))))
        (bind _aswater_1_blueprint_2 (Utilities|Casting|CastToWater1_Blueprint (.HitActor (Collision|BreakHitResult _outhit_2)))
          (:then
            (Variables|Default|SetNearestWater _aswater_1_blueprint_2)
            (Variables|Default|SetbHasValidCondition true :!label _label_2)
            (Default|SetCastType _as_bp_cast_marker_vfx "Purify"))
          (:CastFailed
            (Variables|Default|SetNearestWater 0)
            (bind _asbp_river_2 (Utilities|Casting|CastToBP_River (.HitActor (Collision|BreakHitResult _outhit_2)))
              (:then
                (Variables|Default|SetAs%20BP%20River _asbp_river_2)
                (goto _label_2))
              (:CastFailed
                (Variables|Default|SetAs%20BP%20River 0)
                (Variables|Default|SetbHasValidCondition false)
                (Default|SetCastType _as_bp_cast_marker_vfx "Invalid")))))
        (else
          (Variables|Default|SetNearestWater 0)
          (Variables|Default|SetbHasValidCondition false))))))

(event EventBeginCasting
  (bind _returnvalue (Transformation|GetActorLocation))
  (if (Variables|Default|GetbHasValidCondition)
    (bind _asfirst_person_character (Utilities|Casting|CastToFirstPersonCharacter (Game|GetPlayerCharacter 0)))
    (Utilities|FlowControl|Sequence
      (:then_0
        (Class|BPGenhuInterface|PurifyWater(Message) (Variables|/Game/Blueprints/FirstPersonCharacter.FirstPersonCharacter_C|GetGenhuRef _asfirst_person_character) (Variables|Default|GetNearestWater) _returnvalue)
        (Actor|DestroyActor))
      (:then_1
        (bind _as_bp_river (Variables|Default|GetAs%20BP%20River)
          (:then
            (Class|BPGenhuInterface|PurifyRiver(Message) (Variables|/Game/Blueprints/FirstPersonCharacter.FirstPersonCharacter_C|GetGenhuRef _asfirst_person_character) _as_bp_river _returnvalue))
          (:else))))))

(fn ConstructionScript
  (|CallParentFunction))