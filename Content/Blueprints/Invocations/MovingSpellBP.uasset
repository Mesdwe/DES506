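; MovingSpellBP is a placeable spell that orders the player's Genhu companion to move to the cast marker's location.
; Placement is valid only on flat enough ground, tested by the hit normal's dot with world up, and the marker VFX switches between Move and Invalid.
; A valid cast sends the move to Genhu and destroys the spell.
; Construction caches the marker VFX and clears the Grimoire popup; a SpawnGenhu helper goes uncalled here.
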(event Custom|RemovePopup
  (bind _asfirst_person_character (Utilities|Casting|CastToFirstPersonCharacter (Game|GetPlayerCharacter 0)))
  (Default|RemovePopup (Variables|/Game/Blueprints/FirstPersonCharacter.FirstPersonCharacter_C|GetGrimoireComponent _asfirst_person_character)))

(event EventBeginCasting
  (if (Variables|Default|GetbHasValidCondition)
    (bind _asfirst_person_character (Utilities|Casting|CastToFirstPersonCharacter (Game|GetPlayerCharacter 0)))
    (Class|BPGenhuInterface|MoveGenhuto(Message) (Variables|/Game/Blueprints/FirstPersonCharacter.FirstPersonCharacter_C|GetGenhuRef _asfirst_person_character) (Transformation|GetWorldLocation (Variables|Default|GetCastMarker)))
    (Actor|DestroyActor)))

(event EventSetValidState
  (params (HitResult :type Hit%20Result%20Structure))
  (bind _as_bp_cast_marker_vfx (Variables|Default|GetAs%20BP%20Cast%20Marker%20VFX))
  ;[1 1 1] Update valid state
  (if (< (Math|Vector|DotProduct (.Normal (Collision|BreakHitResult HitResult)) "0.000000,0.000000,1.000000") 0.72)
    (Variables|Default|SetbHasValidCondition false)
    (Default|SetCastType _as_bp_cast_marker_vfx "Invalid")
    (else
      (Variables|Default|SetbHasValidCondition true)
      (Default|SetCastType _as_bp_cast_marker_vfx "Move"))))

(fn ConstructionScript
  (bind _asbp_cast_marker_vfx (Utilities|Casting|CastToBP_CastMarker_VFX (Variables|/Script/Engine.ChildActorComponent|GetChildActor (Variables|Default|GetCastMarker))))
  (Variables|Default|SetAs%20BP%20Cast%20Marker%20VFX _asbp_cast_marker_vfx)
  (CallFunction|RemovePopup))

(fn SpawnGenhu
  (bind _returnvalue (Transformation|GetActorLocation))
  (bind _returnvalue_2 (Game|SpawnActorfromClass "/Game/Blueprints/Genhu_Character.Genhu_Character_C" (Math|Transform|MakeTransform _returnvalue "0, 0, 0" "1,1,1") "AdjustIfPossibleButAlwaysSpawn" 0 0))
  (Transformation|SetActorLocation _returnvalue_2 (+ _returnvalue (Math|Vector|MakeVector 0.0 0.0 (Variables|/Script/Engine.CapsuleComponent|GetCapsuleHalfHeight (Variables|/Script/Engine.Character|GetCapsuleComponent _returnvalue_2)))) false true)
  (return _returnvalue_2))