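; PurifyGenhuBP is a one-shot invocation actor that purifies the player's Genhu.
; On BeginPlay it casts the player character to FirstPersonCharacter and calls PurifySelfMessage on its GenhuRef.
; It then unlocks the non-trigger "Purify Genhu" entry in the character's GrimoireComponent and destroys itself.
; If the cast fails, nothing further runs, including the self-destroy.
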(event EventBeginPlay
  (|CallParentFunction)
  (bind _asfirst_person_character (Utilities|Casting|CastToFirstPersonCharacter (Game|GetPlayerCharacter 0)))
  (Class|BPGenhuInterface|PurifySelf(Message) (Variables|/Game/Blueprints/FirstPersonCharacter.FirstPersonCharacter_C|GetGenhuRef _asfirst_person_character))
  (Default|UnlockInvocationEntry (Variables|/Game/Blueprints/FirstPersonCharacter.FirstPersonCharacter_C|GetGrimoireComponent _asfirst_person_character) "Purify Genhu" false)
  (Actor|DestroyActor))

(event Collision|EventActorBeginOverlap
  (params (OtherActor :type Actor%20Object%20Reference))
  (|CallParentFunction OtherActor) ; This node is disabled and will not be called.\nDrag off pins to build functionality.
)

(event EventTick
  (params (DeltaSeconds :type Float%20%28single-precision%29))
  (|CallParentFunction DeltaSeconds) ; This node is disabled and will not be called.\nDrag off pins to build functionality.
)

(fn ConstructionScript
  (|CallParentFunction))