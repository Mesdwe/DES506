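; PushObjectsBP is the targeting actor for the push invocation, marking which BP_pushable object gets pushed.
; Each tick it moves to where the first-person camera trace hits, or on a miss traces down from the ray's endpoint.
; The hit sets the target, its validity and the cast marker VFX type.
; BeginCasting passes a valid target to the player's GenhuRef via PushingMessage, then destroys the actor.
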(event EventBeginPlay
  (|CallParentFunction)
  (bind _asfirst_person_character (Utilities|Casting|CastToFirstPersonCharacter (Game|GetPlayerCharacter 0)))
  (Variables|Default|SetFirst%20Person%20Camera%20Component (Variables|/Script/Sludge.SludgeCharacter|GetFirstPersonCameraComponent _asfirst_person_character))
  (bind _asbp_cast_marker_vfx (Utilities|Casting|CastToBP_CastMarker_VFX (Variables|/Script/Engine.ChildActorComponent|GetChildActor (Variables|Default|GetCastMarker))))
  (Variables|Default|SetAs%20BP%20Cast%20Marker%20VFX _asbp_cast_marker_vfx))

(event EventTick
  (params (DeltaSeconds :type Float%20%28single-precision%29))
  (bind _first_person_camera_component (Variables|Default|GetFirst%20Person%20Camera%20Component))
  (bind _defaultsceneroot (Variables|Default|GetDefaultSceneRoot))
  (bind _as_bp_cast_marker_vfx (Variables|Default|GetAs%20BP%20Cast%20Marker%20VFX))
  (bind _as_bp_cast_marker_vfx_2 (Variables|Default|GetAs%20BP%20Cast%20Marker%20VFX))
  (bind _returnvalue (Transformation|GetWorldLocation _defaultsceneroot))
  (bind _returnvalue_2 (Transformation|GetWorldLocation _first_person_camera_component))
  (bind _returnvalue_3 (Math|Vector|GetForwardVector _first_person_camera_component))
  (bind _returnvalue_4 (* _returnvalue_3 1e+03))
  (bind _returnvalue_5 (+ _returnvalue_4 _returnvalue_2))
  (|CallParentFunction DeltaSeconds)
  (bind (_outhit _returnvalue_6) (Collision|LineTraceByChannel _returnvalue_2 _returnvalue_5 "TraceTypeQuery1" false 0 "None" true "(R=0.021415,G=0.000000,B=1.000000,A=1.000000)"))
  (if _returnvalue_6
    (Transformation|SetActorLocation (.Location (Collision|BreakHitResult _outhit)) false false)
    (bind _asbp_pushable (Utilities|Casting|CastToBP_pushable (.HitActor (Collision|BreakHitResult _outhit)))
      (:then
        (Variables|Default|SetAs%20BP%20Pushable _asbp_pushable)
        (Variables|Default|SetbHasValidCondition true)
        (Default|SetCastType _as_bp_cast_marker_vfx "Push"))
      (:CastFailed
        (Variables|Default|SetAs%20BP%20Pushable 0)
        (Variables|Default|SetbHasValidCondition false)
        (Default|SetCastType _as_bp_cast_marker_vfx "Invalid")))
    (else
      (Transformation|SetActorLocation _returnvalue_5 false false)
      (bind (_outhit_2 _returnvalue_7) (Collision|LineTraceByChannel _returnvalue (+ _returnvalue (* (Math|Vector|GetUpVector _defaultsceneroot) -1e+03)) "TraceTypeQuery1" false 0 "None"))
      (if _returnvalue_7
        (Transformation|SetActorLocation (.Location (Collision|BreakHitResult _outhit_2)) false false)
        (bind _asbp_pushable_2 (Utilities|Casting|CastToBP_pushable (.HitActor (Collision|BreakHitResult _outhit_2)))
          (:then
            (Variables|Default|SetAs%20BP%20Pushable _asbp_pushable_2)
            (Variables|Default|SetbHasValidCondition true)
            (Default|SetCastType _as_bp_cast_marker_vfx_2 "Push"))
          (:CastFailed
            (Variables|Default|SetAs%20BP%20Pushable 0)
            (Variables|Default|SetbHasValidCondition false)
            (Default|SetCastType _as_bp_cast_marker_vfx_2 "None")))))))

(event EventBeginCasting
  ;[1 1 1] Begin Casting
  (if (Variables|Default|GetbHasValidCondition)
    (bind _asfirst_person_character (Utilities|Casting|CastToFirstPersonCharacter (Game|GetPlayerCharacter 0)))
    (Class|BPGenhuInterface|Pushing(Message) (Variables|/Game/Blueprints/FirstPersonCharacter.FirstPersonCharacter_C|GetGenhuRef _asfirst_person_character) (Variables|Default|GetAs%20BP%20Pushable))
    (Actor|DestroyActor)))

(fn ConstructionScript
  (|CallParentFunction))