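; Spell-casting component that drives four-rune invocations for the player character.
; It opens and closes the casting menu widget, forwarding rune inputs to it and starting and ending staff casting.
; Inputs queue in LoggedArray and play as sequential montages, whose notifies trigger fork, staff and sound effects.
; Each blend-out advances the rune count, calling CastSpell at four, while invalid spells signal GenhuRef and reset casting state.
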(event Custom|ResetAnimSequence
  ;[1 1 1] Play current rune sequence animation
  (Variables|Default|SetIsPlayingAnim false)
  (Variables|Default|SetRuneCount 0)
  (Utilities|Array|Clear (Variables|Default|GetLoggedArray)))

(event Custom|ShowCastingMenu
  (Variables|Default|SetbIsMenuActivated true)
  (Variables|Default|GetCastingMenu
    (:then)
    (:else
      (bind _returnvalue (UserInterface|CreateWidget "/Game/Blueprints/UI/CastingMenu_WID.CastingMenu_WID_C" (Game|GetPlayerController 0)))
      (bind _output_get (Variables|Default|SetCastingMenu _returnvalue))
      (UserInterface|Viewport|AddtoViewport _output_get 0))))

(event Custom|HideCastingMenu
  (if (Variables|Default|GetbIsMenuActivated)
    (Default|ResetRune (Variables|Default|GetCastingMenu))
    (else
      (Variables|Default|GetCastingMenu
        (:then
          (Widget|RemovefromParent (Variables|Default|GetCastingMenu))
          (Variables|Default|SetCastingMenu 0)
          (Variables|Default|SetbIsMenuActivated false))
        (:else)))))

(event Custom|PlayAnimationSequence
  (bind _playerref (Variables|Default|GetPlayerRef))
  (bind _loggedarray (Variables|Default|GetLoggedArray))
  (bind _returnvalue (Transformation|GetActorLocation _playerref))
  ;[1 1 1] Play current rune sequence animation
  (if (not (Variables|Default|GetIsPlayingAnim))
    (Variables|Default|SetIsPlayingAnim true)
    (switch int (Utilities|Array|Get(acopy) (Variables|Default|GetLoggedArray))
      (:0
        (Animation|Montage|PlayMontage (Variables|/Script/Engine.Character|GetMesh (Variables|Default|GetPlayerRef)) "/Game/Blueprints/Animations/shaman_placeholder_Rune1_Anim_Montage.shaman_placeholder_Rune1_Anim_Montage"
          (:OnBlendOut
            (Utilities|Array|RemoveIndex _loggedarray :!label _label)
            (Variables|Default|SetIsPlayingAnim false)
            (CallFunction|IncreaseRuneCount)
            (if (not (== (Utilities|Array|Length _loggedarray) 0))
              (CallFunction|PlayAnimationSequence)))
          (:OnNotifyBegin
            ;;[1 0.9769 0] Fork VFX
            (Default|OnStrike (Variables|/Game/Blueprints/FirstPersonCharacter.FirstPersonCharacter_C|GetForkRef (Variables|Default|GetPlayerRef)))
            (Default|RuneStrike (Variables|/Game/Blueprints/FirstPersonCharacter.FirstPersonCharacter_C|GetStaffRef (Variables|Default|GetPlayerRef)))
            (Audio|PlaySoundatLocation "/Game/Movies/Audio/Tonal_Invocation/sfx_Invoking_01_Cue.sfx_Invoking_01_Cue" _returnvalue "0, 0, 0" 1.0 1.0 0.0 0 0 0))))
      (:1
        (Animation|Montage|PlayMontage (Variables|/Script/Engine.Character|GetMesh (Variables|Default|GetPlayerRef)) "/Game/Blueprints/Animations/shaman_placeholder_Rune2_Anim_Montage.shaman_placeholder_Rune2_Anim_Montage"
          (:OnBlendOut
            (goto _label))
          (:OnNotifyBegin
            ;;[1 0.9769 0] Fork VFX
            (Default|OnStrike (Variables|/Game/Blueprints/FirstPersonCharacter.FirstPersonCharacter_C|GetForkRef (Variables|Default|GetPlayerRef)))
            (Default|RuneStrike (Variables|/Game/Blueprints/FirstPersonCharacter.FirstPersonCharacter_C|GetStaffRef (Variables|Default|GetPlayerRef)) 1)
            (Audio|PlaySoundatLocation "/Game/Movies/Audio/Tonal_Invocation/sfx_Invoking_02_Cue.sfx_Invoking_02_Cue" _returnvalue "0, 0, 0" 1.0 1.0 0.0 0 0 0))))
      (:2
        (Animation|Montage|PlayMontage (Variables|/Script/Engine.Character|GetMesh (Variables|Default|GetPlayerRef)) "/Game/Blueprints/Animations/shaman_placeholder_Rune3_Anim_Montage.shaman_placeholder_Rune3_Anim_Montage"
          (:OnBlendOut
            (goto _label))
          (:OnNotifyBegin
            ;;[1 0.9769 0] Fork VFX
            (Default|OnStrike (Variables|/Game/Blueprints/FirstPersonCharacter.FirstPersonCharacter_C|GetForkRef (Variables|Default|GetPlayerRef)))
            (Default|RuneStrike (Variables|/Game/Blueprints/FirstPersonCharacter.FirstPersonCharacter_C|GetStaffRef (Variables|Default|GetPlayerRef)) 2)
            (Audio|PlaySoundatLocation "/Game/Movies/Audio/Tonal_Invocation/sfx_Invoking_03_Cue.sfx_Invoking_03_Cue" _returnvalue "0, 0, 0" 1.0 1.0 0.0 0 0 0))))
      (:3
        (Animation|Montage|PlayMontage (Variables|/Script/Engine.Character|GetMesh (Variables|Default|GetPlayerRef)) "/Game/Blueprints/Animations/shaman_placeholder_Rune4_Anim_Montage.shaman_placeholder_Rune4_Anim_Montage"
          (:OnBlendOut
            (goto _label))
          (:OnNotifyBegin
            ;;[1 0.9769 0] Fork VFX
            (Default|OnStrike (Variables|/Game/Blueprints/FirstPersonCharacter.FirstPersonCharacter_C|GetForkRef (Variables|Default|GetPlayerRef)))
            (Default|RuneStrike (Variables|/Game/Blueprints/FirstPersonCharacter.FirstPersonCharacter_C|GetStaffRef (Variables|Default|GetPlayerRef)) 3)
            (Audio|PlaySoundatLocation "/Game/Movies/Audio/Tonal_Invocation/sfx_Invoking_04_Cue.sfx_Invoking_04_Cue" _returnvalue "0, 0, 0" 1.0 1.0 0.0 0 0 0)))))))

(event Custom|IncreaseRuneCount
  ;[1 1 1] Play current rune sequence animation
  (Math|Integer|IncrementInt (Variables|Default|GetRuneCount)
    (:%20%20
      (if (>= (Variables|Default|GetRuneCount) 4)
        (Class|SpellComponent|CastSpell)))))

(event EventOnActivateCastingMenu
  (Default|CallActivateCasting)
  (CallFunction|ShowCastingMenu)
  (Default|BeginCasting (Variables|/Game/Blueprints/FirstPersonCharacter.FirstPersonCharacter_C|GetStaffRef (Variables|Default|GetPlayerRef))))

(event EventOnDeactivateCastingMenu
  (Default|CallDeactivateCasting)
  (CallFunction|HideCastingMenu)
  (CallFunction|ResetAnimSequence)
  (Default|EndCasting (Variables|/Game/Blueprints/FirstPersonCharacter.FirstPersonCharacter_C|GetStaffRef (Variables|Default|GetPlayerRef))))

(event EventInvalidSpell
  ;[1 1 1] Invalid spell
  (bind _asfirst_person_character (Utilities|Casting|CastToFirstPersonCharacter (Game|GetPlayerCharacter 0)))
  (bind _genhuref (Variables|/Game/Blueprints/FirstPersonCharacter.FirstPersonCharacter_C|GetGenhuRef _asfirst_person_character)
    (:then
      (Default|SpellError _genhuref)
      (CallFunction|ResetAnimSequence))
    (:else
      _))
  (Variables|Default|SetCurrentSequence "")
  (Variables|Default|SetbIsActivated false)
  (Variables|Default|SetbIsUIActivated false)
  (Variables|Default|SetbIsMenuActivated false)
  (Variables|Default|SetbIsCasting false)
  (Default|CallDeactivateCasting)
  (CallFunction|ResetAnimSequence)
  ;[1 0 0.006121] Temp
  (Utilities|FlowControl|Delay 1.0)
  (CallFunction|HideCastingMenu))

(event EventRune1Behaviour
  ;[1 1 1] Rune Behaviour (called on received input)
  (bind _castingmenu (Variables|Default|GetCastingMenu)
    (:then
      (Default|GetRuneInput _castingmenu "1" 1)
      (Utilities|Array|Add (Variables|Default|GetLoggedArray) 0)
      (CallFunction|PlayAnimationSequence))
    (:else)))

(event EventRune2Behaviour
  ;[1 1 1] Rune Behaviour (called on received input)
  (bind _castingmenu (Variables|Default|GetCastingMenu)
    (:then
      (Default|GetRuneInput _castingmenu "2" 2)
      (Utilities|Array|Add (Variables|Default|GetLoggedArray) 1)
      (CallFunction|PlayAnimationSequence))
    (:else)))

(event EventRune3Behaviour
  ;[1 1 1] Rune Behaviour (called on received input)
  (bind _castingmenu (Variables|Default|GetCastingMenu)
    (:then
      (Default|GetRuneInput _castingmenu "3" 3)
      (Utilities|Array|Add (Variables|Default|GetLoggedArray) 2)
      (CallFunction|PlayAnimationSequence))
    (:else)))

(event EventRune4Behaviour
  ;[1 1 1] Rune Behaviour (called on received input)
  (bind _castingmenu (Variables|Default|GetCastingMenu)
    (:then
      (Default|GetRuneInput _castingmenu "4" 4)
      (Utilities|Array|Add (Variables|Default|GetLoggedArray) 3)
      (CallFunction|PlayAnimationSequence))
    (:else)))

(event EventBeginPlay
  (bind _asfirst_person_character (Utilities|Casting|CastToFirstPersonCharacter (Game|GetPlayerCharacter 0)))
  (Variables|Default|SetPlayerRef _asfirst_person_character))

(event EventImmediatelyCast
  (Variables|Default|SetCurrentSequence "")
  (Variables|Default|SetbIsActivated false)
  (Variables|Default|SetbIsUIActivated false)
  (Variables|Default|SetbIsMenuActivated false)
  (Variables|Default|SetbIsCasting false)
  (Default|CallDeactivateCasting)
  (CallFunction|ResetAnimSequence)
  ;[1 0 0.006121] Temp
  (Utilities|FlowControl|Delay 1.0)
  (CallFunction|HideCastingMenu))

(event EventDelayCast
  ;[1 1 1] Delay cast (move/purify water/push) behaviour
  (Default|CallDeactivateCasting))