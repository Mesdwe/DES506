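; MovingGenhu is a placement marker actor, apparently for a test spell, that follows where the player looks and prints "Select a location" on spawn.
; It caches the FirstPersonCharacter camera, then each tick traces forward along the view and moves to the hit point.
; On a miss it moves to the trace's far end, then traces down from there to snap onto any surface below.
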(event EventBeginPlay
  (|CallParentFunction)
  (Development|PrintString "Select a location" true true "(R=0.000000,G=1.000000,B=0.000000,A=1.000000)")
  (bind _asfirst_person_character (Utilities|Casting|CastToFirstPersonCharacter (Game|GetPlayerCharacter 0)))
  (Variables|Default|SetFirst%20Person%20Camera%20Component (Variables|/Script/Sludge.SludgeCharacter|GetFirstPersonCameraComponent _asfirst_person_character)))

(event Collision|EventActorBeginOverlap
  (params (OtherActor :type Actor%20Object%20Reference))
  (|CallParentFunction OtherActor) ; This node is disabled and will not be called.\nDrag off pins to build functionality.
)

(event EventTick
  (params (DeltaSeconds :type Float%20%28single-precision%29))
  (bind _first_person_camera_component (Variables|Default|GetFirst%20Person%20Camera%20Component))
  (bind _defaultsceneroot (Variables|Default|GetDefaultSceneRoot))
  (bind _returnvalue (Transformation|GetWorldLocation _first_person_camera_component))
  (bind _returnvalue_2 (Math|Vector|GetForwardVector _first_person_camera_component))
  (bind _returnvalue_3 (Transformation|GetWorldLocation _defaultsceneroot))
  (bind _returnvalue_4 (* _returnvalue_2 1e+03))
  (bind _returnvalue_5 (+ _returnvalue_4 _returnvalue))
  (|CallParentFunction DeltaSeconds)
  (bind (_outhit _returnvalue_6) (Collision|LineTraceByChannel _returnvalue _returnvalue_5 "TraceTypeQuery1" false 0 "None" true "(R=0.021415,G=0.000000,B=1.000000,A=1.000000)"))
  (if _returnvalue_6
    (Transformation|SetActorLocation (.Location (Collision|BreakHitResult _outhit)) false false)
    (else
      (Transformation|SetActorLocation _returnvalue_5 false false)
      (bind (_outhit_2 _returnvalue_7) (Collision|LineTraceByChannel _returnvalue_3 (+ _returnvalue_3 (* (Math|Vector|GetUpVector _defaultsceneroot) -1e+03)) "TraceTypeQuery1" false 0 "None"))
      (if _returnvalue_7
        (Transformation|SetActorLocation (.Location (Collision|BreakHitResult _outhit_2)) false false)))))

(fn ConstructionScript
  (|CallParentFunction))