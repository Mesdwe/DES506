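; Cast marker VFX Blueprint that animates two wind swirl effects, fading their opacity and spinning them in opposing directions.
; On BeginPlay, chained timelines drive each swirl's Opacity parameter and both rotations, each timeline started from the previous one's Update.
; Rotation scales with WindRotationSpeed, and the opposite swirl derives its reversed axis from the negated rotation value.
; The construction script creates a dynamic wind swirl material instance for the main swirl only.
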(event EventBeginPlay
  ;[0.4267 1 0.9801] Swirl VFX
  ;;[1 1 1] Fade Swirl in out
  (bind _opacity (Timeline|OpacityFadeInOut Play)
    (:Update
      (Effects|Components|ParticleSystem|SetFloatParameter (Variables|Default|GetWindSwirls) "Opacity" _opacity)
      ;;[1 1 1] Fade Swirl in out opposite swirl
      (bind _opacity_2 (Timeline|OpacityFadeInOuTOpp Play)
        (:Update
          (Effects|Components|ParticleSystem|SetFloatParameter (Variables|Default|GetWindSwirls_Opp) "Opacity" _opacity_2)
          ;;[1 1 1] Rotate Wind Swirls around pivot
          (bind _rotation (Timeline|SwirlRotation Play)
            (:Update
              (Transformation|SetRelativeRotation (Variables|Default|GetWindSwirls) (Math|Vector|RotatorfromAxisandAngle "0.000000,0.000000,1.000000" (* _rotation (Variables|Default|GetWindRotationSpeed))) false false)
              (Transformation|SetRelativeRotation (Variables|Default|GetWindSwirls_Opp) (Math|Vector|RotatorfromAxisandAngle (Math|Vector|MakeVector 0.0 0.0 (* (* _rotation (Variables|Default|GetWindRotationSpeed)) -0.5)) (* _rotation (Variables|Default|GetWindRotationSpeed))) false false))))))))

(fn ConstructionScript
  (Rendering|Material|CreateDynamicMaterialInstance (Variables|Default|GetWindSwirls) 0 "/Game/Art/VFX/Cast-Marker/M_CastMarker_WindSwirl.M_CastMarker_WindSwirl" "None" :!class /Script/Engine.PrimitiveComponent))