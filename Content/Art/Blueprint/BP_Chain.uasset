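; BP_Chain is an art actor that builds a chain of spline mesh segments along its Spline, with no runtime logic.
; The Construction Script multiplies section length and spawn offset by the actor's Y scale, then adds one Y-forward segment per whole section.
; Each segment's start is pulled back by the offset, overlapping the previous one.
; Tangents come from clamped spline locations rather than spline tangents.
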(event EventBeginPlay)

(event Collision|EventActorBeginOverlap
  (params (OtherActor :type Actor%20Object%20Reference)))

(event EventTick
  (params (DeltaSeconds :type Float%20%28single-precision%29)))

(fn ConstructionScript
  (bind _returnvalue (Transformation|GetActorScale3D))
  (bind _spline (Variables|Default|GetSpline))
  ;[0.1714 0.4179 0.04092] Amend values for scale
  (Variables|Default|SetSectionLegnth (* (.y _returnvalue) (Variables|Default|GetSectionLegnth)))
  (Variables|Default|SetSpawnOffset (* (.y _returnvalue) (Variables|Default|GetSpawnOffset)))
  ;[0.05 0.05 0.05] Build mesh loop
  (for _index (range 0 (- (Math|Float|Truncate (/ (Spline|GetSplineLength _spline) (Variables|Default|GetSectionLegnth))) 1))
    (bind _returnvalue_2 (AddComponent|AddSplineMeshComponent false))
    (SplineMesh|SetForwardAxis _returnvalue_2 "Y" true)
    (SplineMesh|SetStartandEnd _returnvalue_2 (Spline|GetLocationatDistanceAlongSpline _spline (- (* _index (Variables|Default|GetSectionLegnth)) (Variables|Default|GetSpawnOffset)) "Local") (Math|Vector|ClampVectorSize (Spline|GetLocationatDistanceAlongSpline _spline (- (* _index (Variables|Default|GetSectionLegnth)) (Variables|Default|GetSpawnOffset)) "Local") 0.0 (Variables|Default|GetSectionLegnth)) (Spline|GetLocationatDistanceAlongSpline _spline (* (+ _index 1) (Variables|Default|GetSectionLegnth)) "Local") (Math|Vector|ClampVectorSize (Spline|GetLocationatDistanceAlongSpline _spline (* (+ _index 1) (Variables|Default|GetSectionLegnth)) "Local") 0.0 (Variables|Default|GetSectionLegnth)) true :!class /Script/Engine.SplineMeshComponent)))