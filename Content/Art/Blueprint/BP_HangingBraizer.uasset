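; BP_HangingBraizer is a hanging brazier actor whose point light flickers like fire.
; BeginPlay seeds the working intensity from the point light's own setting.
; Each Tick samples 1D Perlin noise over accumulated time, scaled by flicker rate and intensity.
; The noise adds to the previous frame's intensity rather than a fixed base, so brightness drifts within a hard-coded clamp range.
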(event EventBeginPlay
  (Variables|Default|SetLightIntensity (Variables|/Script/Engine.LightComponentBase|GetIntensity (Variables|Default|GetPointLight))))

(event Collision|EventActorBeginOverlap
  (params (OtherActor :type Actor%20Object%20Reference)))

(event EventTick
  (params (DeltaSeconds :type Float%20%28single-precision%29))
  ;[1 1 1] Use Noise to control fire point light flicker
  (bind _output_get (Variables|Default|SetTime (+ DeltaSeconds (Variables|Default|GetTime))))
  (bind _output_get_2 (Variables|Default|SetLightIntensity (Math|Float|Clamp(Float) (+ (* (Class|KismetMathLibrary|PerlinNoise1D (* _output_get (Variables|Flicker|GetFlickerRate))) (Variables|Flicker|GetFlickerIntensity)) (Variables|Default|GetLightIntensity)) 5e+03 1.5e+04)))
  (Rendering|Components|Light|SetIntensity (Variables|Default|GetPointLight) _output_get_2))

(fn ConstructionScript)