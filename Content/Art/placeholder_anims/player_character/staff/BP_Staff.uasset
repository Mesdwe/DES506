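; Player's staff actor that displays casting-menu widgets and drives crystal and rune glow effects on its mesh.
; On BeginPlay it binds to the first-person character's spell component, showing or hiding the widgets and ramping crystal glow as the casting menu toggles.
; Controller changes swap widget icons between gamepad and default textures.
; RuneStrike pulses one of four shape runes via timelines writing emissive parameters on a dynamic material instance.
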(event Custom|InitWidget
  (params (IsGamepad :type Boolean))
  ;[1 1 1] Init
  (for (_array_element _array_index) (Components|GetChildrenComponents (Variables|Default|GetWidgets) false)
    (bind _aswidget_component (Utilities|Casting|CastToWidgetComponent _array_element))
    (bind _ascasting_wid (Utilities|Casting|CastToCasting_WID (UserInterface|GetWidget _aswidget_component)))
    (if IsGamepad
      (Appearance|SetBrushfromTexture (Variables|/Game/Blueprints/UI/Casting_WID.Casting_WID_C|GetImage_0 _ascasting_wid) (Utilities|Array|Get(acopy) (Variables|Default|GetControllerCastingWidgets) _array_index) false)
      (else
        (Appearance|SetBrushfromTexture (Variables|/Game/Blueprints/UI/Casting_WID.Casting_WID_C|GetImage_0 _ascasting_wid) (Utilities|Array|Get(acopy) (Variables|Default|GetCastingWidgets) _array_index) false)))))

(event Custom|ShowWidgets
  (for _array_element (Components|GetChildrenComponents (Variables|Default|GetWidgets) false)
    (Rendering|SetVisibility _array_element true false)))

(event Custom|HideWidgets
  (for _array_element (Components|GetChildrenComponents (Variables|Default|GetWidgets) false)
    (Rendering|SetVisibility _array_element false false)))

(event Custom|BeginCasting
  ;[0 0 0] VFX
  ;;[0.3802 0.7727 1] Increase/ Decrease Crystal Glow
  (bind _emissive (Timeline|IncreaseGlow PlayFromStart)
    (:Update
      (Rendering|Material|SetScalarParameterValue (Variables|Default|GetMaterial_Staff) "EmmisiveCrystal" (* _emissive 4.0) :!class /Script/Engine.MaterialInstanceDynamic))))

(event Custom|EndCasting
  ;[0 0 0] VFX
  ;;[0.3802 0.7727 1] Increase/ Decrease Crystal Glow
  (bind _emissive (Timeline|IncreaseGlow ReverseFromEnd)
    (:Update
      (Rendering|Material|SetScalarParameterValue (Variables|Default|GetMaterial_Staff) "EmmisiveCrystal" (* _emissive 4.0) :!class /Script/Engine.MaterialInstanceDynamic))))

(event Custom|RuneStrike
  (params (RuneIndex :type Integer))
  ;[0 0 0] VFX
  ;;[1 1 1] Rune Glow
  (switch int RuneIndex
    (:0
      (bind _emissive_value (Timeline|x_Rune_Glow PlayFromStart)
        (:Update
          ;;;[0.5452 0.8477 1] X
          (Rendering|Material|SetScalarParameterValue (Variables|Default|GetMaterial_Staff) "EmmisiveX" (+ (* _emissive_value (Variables|Runes|GetRuneStrikeEmissive)) (Variables|Runes|GetRuneIdleEmissive)) :!class /Script/Engine.MaterialInstanceDynamic))))
    (:1
      (bind _emissive_value_2 (Timeline|Circle_Rune_Glow PlayFromStart)
        (:Update
          ;;;[1 0.5646 0.4947] Circle
          (Rendering|Material|SetScalarParameterValue (Variables|Default|GetMaterial_Staff) "EmmisiveO" (+ (* _emissive_value_2 (Variables|Runes|GetRuneStrikeEmissive)) (Variables|Runes|GetRuneIdleEmissive)) :!class /Script/Engine.MaterialInstanceDynamic))))
    (:2
      (bind _emissive_value_3 (Timeline|triangle_Rune_Glow PlayFromStart)
        (:Update
          ;;;[0.5528 1 0.4499] Triangle
          (Rendering|Material|SetScalarParameterValue (Variables|Default|GetMaterial_Staff) "EmmisiveTriangle" (+ (* _emissive_value_3 (Variables|Runes|GetRuneStrikeEmissive)) (Variables|Runes|GetRuneIdleEmissive)) :!class /Script/Engine.MaterialInstanceDynamic))))
    (:3
      (bind _emissive_value_4 (Timeline|square__Rune_Glow PlayFromStart)
        (:Update
          ;;;[0.9986 0.6641 1] Square
          (Rendering|Material|SetScalarParameterValue (Variables|Default|GetMaterial_Staff) "EmmisiveSquare" (+ (* _emissive_value_4 (Variables|Runes|GetRuneStrikeEmissive)) (Variables|Runes|GetRuneIdleEmissive)) :!class /Script/Engine.MaterialInstanceDynamic))))))

(event EventBeginPlay
  (CallFunction|SetInitialMaterialParameters)
  (CallFunction|InitWidget false)
  (bind _asfirst_person_character (Utilities|Casting|CastToFirstPersonCharacter (Game|GetPlayerCharacter 0)))
  (EventDispatchers|BindEventtoOnActivateCastingMenu (Variables|/Game/Blueprints/FirstPersonCharacter.FirstPersonCharacter_C|GetSpellComponentBP _asfirst_person_character) (delegate Custom|ShowWidgets))
  (EventDispatchers|BindEventtoOnDeactivateCastingMenu (Variables|/Game/Blueprints/FirstPersonCharacter.FirstPersonCharacter_C|GetSpellComponentBP _asfirst_person_character) (delegate Custom|HideWidgets))
  (EventDispatchers|BindEventtoOnActivateCastingMenu (Variables|/Game/Blueprints/FirstPersonCharacter.FirstPersonCharacter_C|GetSpellComponentBP _asfirst_person_character) (delegate Custom|BeginCasting))
  (EventDispatchers|BindEventtoOnDeactivateCastingMenu (Variables|/Game/Blueprints/FirstPersonCharacter.FirstPersonCharacter_C|GetSpellComponentBP _asfirst_person_character) (delegate Custom|EndCasting))
  (EventDispatchers|BindEventtoOnControllerChange _asfirst_person_character (delegate Custom|InitWidget))
  (CallFunction|HideWidgets))

(fn ConstructionScript
  (bind _returnvalue (Rendering|Material|CreateDynamicMaterialInstance (Variables|Default|GetSkeletalMesh) 0 "/Game/Art/characters/Staff/Mi_Staff.Mi_Staff" "None" :!class /Script/Engine.PrimitiveComponent))
  (Variables|Default|SetMaterial_Staff _returnvalue))

(fn SetInitialMaterialParameters
  (bind _runeidleemissive (Variables|Runes|GetRuneIdleEmissive))
  ;[0.5452 0.8477 1] X
  (Rendering|Material|SetScalarParameterValue (Variables|Default|GetMaterial_Staff) "EmmisiveX" _runeidleemissive :!class /Script/Engine.MaterialInstanceDynamic)
  ;[1 0.5646 0.4947] Circle
  (Rendering|Material|SetScalarParameterValue (Variables|Default|GetMaterial_Staff) "EmmisiveO" _runeidleemissive :!class /Script/Engine.MaterialInstanceDynamic)
  ;[0.5528 1 0.4499] Triangle
  (Rendering|Material|SetScalarParameterValue (Variables|Default|GetMaterial_Staff) "EmmisiveTriangle" _runeidleemissive :!class /Script/Engine.MaterialInstanceDynamic)
  ;[0.9986 0.6641 1] Square
  (Rendering|Material|SetScalarParameterValue (Variables|Default|GetMaterial_Staff) "EmmisiveSquare" _runeidleemissive :!class /Script/Engine.MaterialInstanceDynamic))